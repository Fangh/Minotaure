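; Minotaur dialog character that acts as both the game's opening gatekeeper and its losing ending, depending on whether any buildings were destroyed.
; StartDialog plays the normal or losing dialog with the character's avatar, based on the BuildingDestroyed count.
; Finish either shows a HUD with the destruction percentage out of ten buildings and quits after a delay, or re-enables first-person character input and removes the StartDoor actors.
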(event `StartDialog`
  (if (> (`self.BuildingDestroyed`) 0)
    (`self.CharacterDialog` (`self.DialogLoose`) (`self.Avatar`))
    (else
      (`self.CharacterDialog` (`self.Dialog`) (`self.Avatar`)))))

(event `Finish`
  (bind _buildingdestroyed (`self.BuildingDestroyed`))
  (if (> _buildingdestroyed 0)
    (bind _returnvalue (`|CreateWidget` "/Game/BluePrints/LostHUD.LostHUD_C"))
    (set `/Game/BluePrints/LostHUD.PercentDestroyed` (`KismetTextLibrary.Conv_DoubleToText` (* (/ (`KismetMathLibrary.Conv_IntToDouble` _buildingdestroyed) 10.0) 100.0) "HalfToEven" true 1 3 0 0) _returnvalue)
    (`UserWidget.AddToViewport` _returnvalue 0)
    (`KismetSystemLibrary.Delay` 5.0)
    (`KismetSystemLibrary.QuitGame` null "Quit")
    (else
      (bind _outactors (`GameplayStatics.GetAllActorsOfClass` "/Game/FirstPersonBP/Blueprints/FirstPersonCharacter.FirstPersonCharacter_C"))
      (for _array_element _outactors
        (`self.EnableInput` _array_element null)
        (bind _outactors_2 (`GameplayStatics.GetAllActorsOfClass` "/Game/BluePrints/StartDoor.StartDoor_C"))
        (`self.K2_DestroyActor` _outactors_2)))))

(fn `UserConstructionScript`
  (`parent.UserConstructionScript`))