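; MovingWall is a wall actor that slides between front, middle and back positions along its right vector.
; Move asks ChooseNextPos for the adjacent slot, then a timeline lerps the location while a gate blocks new moves until it finishes.
; Up and Down keys trigger Move for debugging.
; Select attaches a particle beam that Tick stretches from the selecting source to the wall, and UnSelect destroys it.
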(event `Key|Up`
  (params (Key :type "Key Structure" :default "AnyKey"))
  ;[1 1 1] Debug
  (:`Pressed`
    (`self.Move` "NewEnumerator0")))

(event `Key|Down`
  (params (Key :type "Key Structure" :default "AnyKey"))
  ;[1 1 1] Debug
  (:`Pressed`
    (`self.Move` "NewEnumerator1")))

(event `self.ReceiveBeginPlay`
  ;[1 1 1] Init
  (set `self.Forward` (`self.GetActorRightVector`))
  (set `self.MiddleLocation` (`self.K2_GetActorLocation`))
  (set `self.CurrentPos` "NewEnumerator1")
  ;[1 1 1] Debug
  (`self.EnableInput` (`GameplayStatics.GetPlayerController` 0)))

(event `Move`
  (params (Direction :type "/Game/BluePrints/PistolDirection Enum"))
  ;[1 1 1] Movement Behavior
  (`/Engine/EditorBlueprintResources/StandardMacros.Gate` false :!label _label
    (:`Exit`
      (`|ExecutionSequence`
        (:`then_0`
          (goto _label :!via `Close`))
        (:`then_1`
          ;;[1 1 1] set differents positions variable to move
          (bind (_nextlocation _nextpos) (`self.ChooseNextPos` Direction))
          (set `self.NextLocation` _nextlocation)
          (set `self.CurrentLocation` (`self.K2_GetActorLocation`))
          ;;[1 1 1] Move
          (bind (_direction _curve) (`Timeline|MoveTimeline` :!via `PlayFromStart`)
            (:`Update`
              (`self.K2_SetActorLocation` (`KismetMathLibrary.VLerp` (`self.CurrentLocation`) (`self.NextLocation`) _curve)))
            (:`Finished`
              (set `self.CurrentPos` _nextpos)
              (goto _label :!via `Open`))))))))

(event `Select`
  (params (SourcePawn :type "SphereComponent Object Reference"))
  ;[1 1 1] Player click on me
  (set `self.Source` SourcePawn)
  (bind _returnvalue (`AddComponent|NODE_AddParticleSystemComponent-0`))
  (set `self.Beam` _returnvalue))

(event `self.ReceiveTick`
  (params (DeltaSeconds :type "Float (single-precision)"))
  (bind _beam (`self.Beam`))
  ;[1 1 1] Set Beam + Check player Distance
  (`/Engine/EditorBlueprintResources/StandardMacros.IsValid` _beam
    (:`Is Valid`
      (`ParticleSystemComponent.SetBeamSourcePoint` _beam 0 (`SceneComponent.K2_GetComponentLocation` (`self.Source`)) 0)
      (`ParticleSystemComponent.SetBeamTargetPoint` _beam 0 (`self.K2_GetActorLocation`) 0))))

(event `UnSelect`
  (bind _beam (`self.Beam`))
  ;[1 1 1] Player release click
  (`/Engine/EditorBlueprintResources/StandardMacros.IsValid` _beam
    (:`Is Valid`
      (`ActorComponent.K2_DestroyComponent` _beam)
      (bind _output_get (set `self.Beam` null))
      (`KismetSystemLibrary.PrintString` (`KismetSystemLibrary.GetDisplayName` _output_get)))))

(fn `ChooseNextPos`
  (params (Direction :type "/Game/BluePrints/PistolDirection Enum"))
  (returns (NextLocation :type "Vector Structure") (NextPos :type "/Game/BluePrints/WallPos Enum"))
  (bind _returnvalue (* (`self.Forward`) 190.0))
  (`|ExecutionSequence`
    (:`then_0`
      (if (and (`|EnumEquality` (`self.CurrentPos`) "NewEnumerator0") (`|EnumEquality` Direction "NewEnumerator1"))
        (return (`self.MiddleLocation`) "NewEnumerator1")))
    (:`then_1`
      (if (and (`|EnumEquality` (`self.CurrentPos`) "NewEnumerator2") (`|EnumEquality` Direction "NewEnumerator0"))
        (return (`self.MiddleLocation`) "NewEnumerator1")))
    (:`then_2`
      (if (and (`|EnumEquality` (`self.CurrentPos`) "NewEnumerator1") (`|EnumEquality` Direction "NewEnumerator0"))
        (return (+ (`self.MiddleLocation`) _returnvalue) "NewEnumerator0")))
    (:`then_3`
      (if (and (`|EnumEquality` (`self.CurrentPos`) "NewEnumerator1") (`|EnumEquality` Direction "NewEnumerator1"))
        (return (- (`self.MiddleLocation`) _returnvalue) "NewEnumerator2")))))

(fn `UserConstructionScript`)